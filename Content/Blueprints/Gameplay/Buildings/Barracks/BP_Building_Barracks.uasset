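; Barracks building that queues and spawns the units available to its clan.
; BeginPlay creates a queue entry per clan unit class; DeployUnit increments that entry's count and starts a looping timer.
; Each tick advances all pending classes in parallel, spawning at UnitSpawnLocation when TimeToDeploy, read from class defaults, elapses.
; DeployingData's OnRep broadcasts progress; the timer clears only if that array is empty, not when counts reach zero.
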(event EventBeginPlay
  (|CallParentFunction)
  (for _array_element (.unitclasses (.Value (Utilities|Map|Find (Variables|Default|GetUnits) (Variables|Default|GetClan))))
    (Utilities|Array|Add (Variables|Default|GetDeployingData) (Utilities|Struct|MakeST_BarracksDeployingData _array_element 0 0.0))))

(fn ConstructionScript
  (|CallParentFunction))

(fn DeployUnit
  (params (UnitClass :type BP%20Master%20Unit%20Class%20Reference))
  (for (_array_element _array_index) (Variables|Default|GetDeployingData)
    (if (== (.unitclass _array_element) UnitClass)
      (bind _structout (Utilities|Struct|SetmembersinST_BarracksDeployingData (Utilities|Array|Get(acopy) (Variables|Default|GetDeployingData) _array_index) (+ (.Remaining (Utilities|Struct|BreakST_BarracksDeployingData (Utilities|Array|Get(acopy) (Variables|Default|GetDeployingData) _array_index))) 1)))
      (Utilities|Array|SetArrayElem (Variables|Default|GetDeployingData) _array_index _structout)))
  (if (not (Utilities|Time|IsValidTimerHandle (Variables|Default|GetDeployingTimer)))
    (bind _returnvalue (Utilities|Time|SetTimerbyEvent (EventDispatchers|CreateEvent :!event DeployingHandle) 0.1 true))
    (Variables|Default|SetDeployingTimer _returnvalue)))

(fn OnRepDeployingData
  (Default|CallUpdatedDeploying (Variables|Default|GetDeployingData)))

(fn DeployingHandle
  (bind _output_get (LocalVariables|SetDeployingDataTemp (Variables|Default|GetDeployingData)))
  (for (_array_element _array_index) _output_get
    (if (> (.remaining _array_element) 0)
      (if (>= (+ (.currenttime _array_element) 0.1) (.TimeToDeploy (Utilities|GetClassDefaults (.unitclass _array_element))))
        (CallFunction|SpawnUnit (.unitclass _array_element))
        (bind _structout (Utilities|Struct|SetmembersinST_BarracksDeployingData (Utilities|Array|Get(acopy) (LocalVariables|GetDeployingDataTemp) _array_index) (- (.remaining _array_element) 1) 0.0))
        (Utilities|Array|SetArrayElem (LocalVariables|GetDeployingDataTemp) _array_index _structout)
        (else
          (bind _structout_2 (Utilities|Struct|SetmembersinST_BarracksDeployingData (Utilities|Array|Get(acopy) (LocalVariables|GetDeployingDataTemp) _array_index) (+ (.currenttime _array_element) 0.1)))
          (Utilities|Array|SetArrayElem (LocalVariables|GetDeployingDataTemp) _array_index _structout_2)))))
  (bind _output_get_2 (Variables|Default|SetDeployingData (LocalVariables|GetDeployingDataTemp)))
  (if (== (Utilities|Array|Length _output_get_2) 0)
    (Utilities|Time|ClearandInvalidateTimerbyHandle (Variables|Default|GetDeployingTimer)))
  (return))

(fn SpawnUnit
  (params (UnitClass :type BP%20Master%20Unit%20Class%20Reference))
  (Game|SpawnActorfromClass UnitClass (Math|Transform|MakeTransform (Transformation|GetWorldLocation (Variables|Default|GetUnitSpawnLocation)) "0, 0, 0" "1,1,1") "AdjustIfPossibleButAlwaysSpawn" 0 0))

(fn GetLocalUnits
  (bind _aspc_gameplay (Utilities|Casting|CastToPC_Gameplay (Game|GetPlayerController 0)))
  (return (.unitclasses (.Value (Utilities|Map|Find (Variables|Default|GetUnits) (Variables|/Game/Blueprints/Gameplay/GameMode/PC_Gameplay.PC_Gameplay_C|GetClan _aspc_gameplay))))))