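; BP_Building_Pestle is a clan-owned building that periodically generates gold for its owning clan.
; On BeginPlay, only the authority starts a looping five-second timer, stored as GiveGoldTimer, to drive the payouts.
; GiveGold adds gold to the clan's player controller, found through GM_Gameplay.
; The payout is the base amount at level one, then grows in whole multiples of it via a truncated level multiplier.
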(event Custom|GiveGold
  (bind _asgm_gameplay (Utilities|Casting|CastToGM_Gameplay (Game|GetGameMode)))
  (Variables|/Game/Blueprints/Gameplay/GameMode/PC_Gameplay.PC_Gameplay_C|SetGold (Default|GetPCOfClan _asgm_gameplay (Variables|Default|GetClan)) (+ (Variables|/Game/Blueprints/Gameplay/GameMode/PC_Gameplay.PC_Gameplay_C|GetGold (Default|GetPCOfClan _asgm_gameplay (Variables|Default|GetClan))) (select (== (Variables|Default|GetLevel) 1) (Variables|Default|GetDefaultGoldAmount) (+ (Variables|Default|GetDefaultGoldAmount) (* (Variables|Default|GetDefaultGoldAmount) (Math|Float|Truncate (* (- (Variables|Default|GetLevel) 1) (Variables|Default|GetGoldLevelMultiplier)))))))))

(event EventBeginPlay
  (|CallParentFunction)
  (Networking|SwitchHasAuthority
    (:Authority
      (bind _returnvalue (Utilities|Time|SetTimerbyEvent (EventDispatchers|CreateEvent :!event Custom|GiveGold) 5.0 true))
      (Variables|Default|SetGiveGoldTimer _returnvalue))))

(fn ConstructionScript
  (|CallParentFunction))