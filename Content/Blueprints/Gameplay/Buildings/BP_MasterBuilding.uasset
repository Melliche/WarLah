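; Base building actor for a clan-based game, with health, selection highlighting colored by friend or enemy, leveling, and optional turret defense.
; Damage lowers replicated health and destroys the building at zero, while a 3D health widget updates via OnRep and faces the camera on non-dedicated-server instances.
; On the authority, defending buildings track the nearest enemy unit through collision overlaps and use a looping timer to fire projectiles at it.
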(event OnComponentBeginOverlap(AttackCollision)
  (params (OverlappedComponent :type Primitive%20Component%20Object%20Reference) (OtherActor :type Actor%20Object%20Reference) (OtherComp :type Primitive%20Component%20Object%20Reference) (OtherBodyIndex :type Integer) (bFromSweep :type Boolean) (SweepResult :type Hit%20Result%20Structure%20%28by%20ref%29))
  (bind _returnvalue (Transformation|GetActorLocation))
  ;[1 1 1] Handles starting to attack when possible
  (Networking|SwitchHasAuthority
    (:Authority
      (if (Variables|Default|GetDefends)
        (bind _asbp_master_unit (Utilities|Casting|CastToBP_MasterUnit OtherActor))
        (if (Utilities|Enum|NotEqual(Enum) (Variables|/Game/Blueprints/Gameplay/Units/BP_MasterUnit.BP_MasterUnit_C|GetClan _asbp_master_unit) (Variables|Default|GetClan))
          (bind _currentattacktarget (Variables|Default|GetCurrentAttackTarget)
            (:then
              (if (< (Math|Vector|Distance(Vector) _returnvalue (Transformation|GetActorLocation _asbp_master_unit)) (Math|Vector|Distance(Vector) (Transformation|GetActorLocation _currentattacktarget) _returnvalue))
                (Variables|Default|SetCurrentAttackTarget _asbp_master_unit)))
            (:else
              (Variables|Default|SetCurrentAttackTarget _asbp_master_unit)
              (bind _returnvalue_2 (Utilities|Time|SetTimerbyEvent (EventDispatchers|CreateEvent :!event Custom|Attack) (Variables|Default|GetAttackRate) true))
              (Variables|Default|SetAttackTimer _returnvalue_2))))))))

(event OnComponentEndOverlap(AttackCollision)
  (params (OverlappedComponent :type Primitive%20Component%20Object%20Reference) (OtherActor :type Actor%20Object%20Reference) (OtherComp :type Primitive%20Component%20Object%20Reference) (OtherBodyIndex :type Integer))
  ;[1 1 1] Handles stopping to attack when possible
  (Networking|SwitchHasAuthority
    (:Authority
      (bind _asbp_master_unit (Utilities|Casting|CastToBP_MasterUnit OtherActor))
      (if (== _asbp_master_unit (Variables|Default|GetCurrentAttackTarget))
        (bind (_found _targetunit) (CallFunction|FindClosestAttackTarget))
        (if _found
          (Variables|Default|SetCurrentAttackTarget _targetunit)
          (else
            (Utilities|Time|ClearandInvalidateTimerbyHandle (Variables|Default|GetAttackTimer))
            (Variables|Default|SetCurrentAttackTarget 0)))))))

(event Custom|UpdateHealth
  ;[1 1 1] Handles updating the health widget
  (bind _aswbp_health_3d (Utilities|Casting|CastToWBP_Health3D (UserInterface|GetUserWidgetObject (Variables|Default|GetHealthWidget))))
  (Default|UpdateHealth _aswbp_health_3d (Variables|Default|GetCurrentHealth) (Variables|Default|GetMaxHealth)))

(event Custom|Attack
  (bind _turretlocation (Variables|Default|GetTurretLocation))
  (bind _returnvalue (Transformation|GetWorldLocation _turretlocation))
  ;[1 1 1] Handles spawning projectile
  (Game|SpawnActorfromClass (Variables|Default|GetProjectileClass) (Math|Transform|MakeTransform _returnvalue (Math|Rotator|FindLookatRotation _returnvalue (Transformation|GetActorLocation (Variables|Default|GetCurrentAttackTarget))) "1,1,1") "Undefined" self (Variables|Default|GetDamage) (Variables|Default|GetCurrentAttackTarget) 0))

(event Game|Damage|EventAnyDamage
  (params (Damage :type Float%20%28single-precision%29) (DamageType :type Damage%20Type%20Object%20Reference) (InstigatedBy :type Controller%20Object%20Reference) (DamageCauser :type Actor%20Object%20Reference))
  ;[1 1 1] Handles receiving damage and destroying itself when no health
  (bind _output_get (Variables|Default|SetCurrentHealth (Math|Float|Clamp(Float) (- (Variables|Default|GetCurrentHealth) Damage) 0.0 (Variables|Default|GetMaxHealth))))
  (if (== _output_get 0.0)
    (Actor|DestroyActor)))

(event EventTick
  (params (DeltaSeconds :type Float%20%28single-precision%29))
  (bind _healthwidget (Variables|Default|GetHealthWidget))
  ;[1 1 1] Handles rotating health widget towards camera when possible (If not dedicated server)
  (Networking|CanExecuteCosmeticEvents
    (:True
      (Transformation|SetWorldRotation _healthwidget (Math|Rotator|FindLookatRotation (Transformation|GetWorldLocation _healthwidget) (Transformation|GetActorLocation (Game|GetPlayerCameraManager 0))) false false))))

(event EventBeginPlay
  ;[1 1 1] Init
  (Networking|CanExecuteCosmeticEvents
    (:True
      (CallFunction|UpdateHealth))))

(fn ConstructionScript)

(fn OnRepCurrentHealth
  (Networking|CanExecuteCosmeticEvents
    (:True
      (CallFunction|UpdateHealth))))

(fn IsFriendly
  (params (PC :type PC%20Gameplay%20Object%20Reference))
  (return (Utilities|Enum|Equal(Enum) (Variables|/Game/Blueprints/Gameplay/GameMode/PC_Gameplay.PC_Gameplay_C|GetClan PC) (Variables|Default|GetClan))))

(fn FindClosestAttackTarget
  (for (_array_element _array_index) (Collision|GetOverlappingActors (Variables|Default|GetAttackCollision) "/Game/Blueprints/Gameplay/Units/BP_MasterUnit.BP_MasterUnit_C" :!class /Script/Engine.PrimitiveComponent)
    (bind _asbp_master_unit (Utilities|Casting|CastToBP_MasterUnit _array_element))
    (if (Utilities|Enum|NotEqual(Enum) (Variables|/Game/Blueprints/Gameplay/Units/BP_MasterUnit.BP_MasterUnit_C|GetClan _asbp_master_unit) (Variables|Default|GetClan))
      (if (or (== _array_index 0) (< (Math|Vector|Distance(Vector) (Transformation|GetActorLocation _array_element) (Transformation|GetActorLocation)) (LocalVariables|GetClosestDistance)))
        (LocalVariables|SetClosestUnit _asbp_master_unit)
        (LocalVariables|SetClosestDistance (Math|Vector|Distance(Vector) (Transformation|GetActorLocation _array_element) (Transformation|GetActorLocation))))))
  (return (Utilities|IsValid (LocalVariables|GetClosestUnit)) (LocalVariables|GetClosestUnit)))

(fn ToggleSelection
  (params (Show :type Boolean))
  (bind _output_get (Variables|Default|SetIsSelected Show))
  (if _output_get
    (Rendering|Material|SetMaterial (Variables|Default|GetSelectionMesh) 0 (select (CallFunction|IsFriendly (.AsPC%20Gameplay (Utilities|Casting|CastToPC_Gameplay (Game|GetPlayerController 0)))) "/Game/Materials/M_SelectedUnit_Friendly.M_SelectedUnit_Friendly" "/Game/Materials/M_SelectedUnit_Enemy.M_SelectedUnit_Enemy")))
  (Rendering|SetVisibility (Variables|Default|GetSelectionMesh) (Variables|Default|GetIsSelected) false))

(fn StartAction
  (params (BuildingAction :type BP%20Master%20Building%20Action%20Class%20Reference)))

(fn LevelUp
  (Math|Integer|IncrementInt (Variables|Default|GetLevel)))

(fn GetClan
  (return (Variables|Default|GetClan)))

(fn GetInteractionDistance
  (return 2.5e+02))

(fn IsDead
  (return false))