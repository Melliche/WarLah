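; BP_CameraPawn is the player-controlled camera pawn that moves, rotates and zooms the gameplay view.
; Axis inputs offset the pawn along its forward and right vectors and yaw it in world space, scaled by speed and delta time.
; Zoom presses shift the camera's relative height within clamped limits through CameraZoom.
; The Pause action toggles the pause menu through the HUD reference on PC_Gameplay.
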(event Custom|CameraZoom
  (params (Value :type Float%20%28single-precision%29))
  (bind _camera (Variables|Default|GetCamera))
  (bind _relativelocation (Variables|/Script/Engine.SceneComponent|GetRelativeLocation _camera))
  ;[1 1 1] Zoom in/out
  (Transformation|SetRelativeLocation _camera (Math|Vector|MakeVector (.x _relativelocation) (.y _relativelocation) (Math|Float|Clamp(Float) (+ (.z _relativelocation) (* Value (Variables|Default|GetZoomSensitivity) (Utilities|Time|GetWorldDeltaSeconds))) 6.5e+02 1.65e+03)) false false))

(event Input|ActionEvents|InputActionZoomIn
  (params (Key :type Key%20Structure :default "None"))
  ;[1 1 1] Zoom in/out
  (:Pressed
    (CallFunction|CameraZoom -1.0)))

(event Input|ActionEvents|InputActionZoomOut
  (params (Key :type Key%20Structure :default "None"))
  ;[1 1 1] Zoom in/out
  (:Pressed
    (CallFunction|CameraZoom 1.0)))

(event Input|ActionEvents|InputActionPause
  (params (Key :type Key%20Structure :default "None"))
  ;[1 1 1] Pause input
  (:Pressed
    (Default|TogglePauseMenu (Default|GetHUDRef (.AsPC%20Gameplay (Utilities|Casting|CastToPC_Gameplay (Game|GetPlayerController 0)))))))

(event Input|AxisEvents|InputAxisMoveForward
  (params (AxisValue :type Float%20%28single-precision%29))
  ;[1 1 1] Camera movement
  (Transformation|AddActorWorldOffset (* (Transformation|GetActorForwardVector) (* (Variables|Default|GetMovementSpeed) AxisValue (Utilities|Time|GetWorldDeltaSeconds)))))

(event Input|AxisEvents|InputAxisMoveRight
  (params (AxisValue :type Float%20%28single-precision%29))
  ;[1 1 1] Camera movement
  (Transformation|AddActorWorldOffset (* (Transformation|GetActorRightVector) (* (Variables|Default|GetMovementSpeed) AxisValue (Utilities|Time|GetWorldDeltaSeconds)))))

(event Input|AxisEvents|InputAxisRotate
  (params (AxisValue :type Float%20%28single-precision%29))
  ;[1 1 1] Rotate
  (Class|Actor|AddActorWorldRotation (Math|Rotator|MakeRotator 0.0 0.0 (* (Variables|Default|GetRotationSpeed) AxisValue (Utilities|Time|GetWorldDeltaSeconds)))))

(fn ConstructionScript)