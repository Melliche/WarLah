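; RTS player controller that handles unit and building selection, move and attack commands, building construction and end/waiting screens.
; A timer separates click selection from drag selection, which resizes a box actor in camera-relative space from cursor traces.
; Construction mode moves a ghost with the cursor until click release requests a build.
; Server events execute commands and gold-checked builds and deployments, while OnRep functions broadcast gold and building-list updates.
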(event Custom|StartMultiSelection
  ;[1 1 1] Starts multi selection, spawns selection box
  (Utilities|Time|ClearandInvalidateTimerbyHandle (Variables|Default|GetMultiSelectionTimer))
  (Variables|Default|SetIsMultiSelection true)
  (bind (_location _sizex _sizey) (CallFunction|GetNewMultiSelectionData))
  (bind _returnvalue (Game|SpawnActorfromClass "/Game/Blueprints/Gameplay/GameMode/BP_MultiSelectionBoxd.BP_MultiSelectionBoxd_C" (Math|Transform|MakeTransform _location (Transformation|GetActorRotation (CallFunction|GetCameraPawn)) "1,1,1") "Undefined" 0 0))
  (Variables|Default|SetMultiSelectionBox _returnvalue)
  (Components|Box|SetBoxExtent (Variables|/Game/Blueprints/Gameplay/GameMode/BP_MultiSelectionBoxd.BP_MultiSelectionBoxd_C|GetBox _returnvalue) (Math|Vector|MakeVector _sizex _sizey 5e+02) true)
  (Transformation|AttachActorToActor _returnvalue (CallFunction|GetCameraPawn) "None" "KeepWorld" "KeepWorld" "KeepWorld" true))

(event Custom|SingleSelection
  ;[1 1 1] Handles single selection logic for units and buildings
  (CallFunction|UnselectAllUnits)
  (CallFunction|UnselectBuilding)
  (bind _hitactor (CallFunction|GetMouseHitActor))
  (bind _asbp_master_unit (Utilities|Casting|CastToBP_MasterUnit _hitactor)
    (:then
      (CallFunction|SelectUnits (Utilities|Array|MakeArray _asbp_master_unit)))
    (:CastFailed
      (bind _asbp_master_building (Utilities|Casting|CastToBP_MasterBuilding _hitactor))
      (CallFunction|SelectBuilding _asbp_master_building))))

(event Custom|ToggleConstruction
  (params (Show :type Boolean) (BuildingClass :type BP%20Master%20Building%20Class%20Reference))
  ;[1 1 1] Toggles construction mode
  (bind _output_get (Variables|Default|SetIsConstructionMode Show))
  (if _output_get
    (Variables|Default|SetBuildingClass BuildingClass)
    (bind _hitlocation (CallFunction|GetMouseHitLocation))
    (bind _returnvalue (Game|SpawnActorfromClass "/Game/Blueprints/Gameplay/Buildings/BP_BuildingGhost.BP_BuildingGhost_C" (Math|Transform|MakeTransform _hitlocation "0, 0, 0" "1,1,1") "Undefined" 0 (.GhostMesh (Utilities|GetClassDefaults (Variables|Default|GetBuildingClass))) 0))
    (Variables|Default|SetBuildingGhost _returnvalue)
    (else
      (bind _buildingghost (Variables|Default|GetBuildingGhost)
        (:then
          (Actor|DestroyActor _buildingghost))
        (:else
          _))
      (Variables|Default|SetBuildingGhost 0)
      (Variables|Default|SetBuildingClass 0))))

(event Custom|ConstructionTick
  ;[1 1 1] Construction tick to update the building ghost location
  (if (Variables|Default|GetIsConstructionMode)
    (bind _buildingghost (Variables|Default|GetBuildingGhost)
      (:then
        (bind _hitlocation (CallFunction|GetMouseHitLocation))
        (Transformation|SetActorLocation _buildingghost _hitlocation false false))
      (:else))))

(event Custom|ServerBuild
  (params (Building :type BP%20Master%20Building%20Class%20Reference) (Location :type Vector))
  (bind _cost (Utilities|GetClassDefaults Building))
  ;[1 1 1] Server event to build building if gold enough
  (if (>= (Utilities|Array|FindItem (Variables|Default|GetConstructionBuildings) Building) 0)
    (if (>= (Variables|Default|GetGold) _cost)
      (Variables|Default|SetGold (- (Variables|Default|GetGold) _cost))
      (Game|SpawnActorfromClass Building (Math|Transform|MakeTransform Location "0, 0, 0" "1,1,1") "Undefined" 0 (Variables|Default|GetClan) 0))))

(event Custom|ServerRequestDeployUnit
  (params (Barracks :type BP%20Building%20Barracks%20Object%20Reference) (UnitClass :type BP%20Master%20Unit%20Class%20Reference))
  (bind _cost (Utilities|GetClassDefaults UnitClass))
  ;[1 1 1] Server event to request deploy unit on barracks
  (if (>= (Variables|Default|GetGold) _cost)
    (Variables|Default|SetGold (- (Variables|Default|GetGold) _cost))
    (Default|DeployUnit Barracks UnitClass)))

(event Custom|ClientToggleWaitingScreen
  (params (Show :type Boolean))
  ;[1 1 1] Client toggles waiting screen
  (Default|ToggleWaitingScreen (CallFunction|GetHUDRef) Show))

(event Custom|StopMultiSelection
  ;[1 1 1] End of multiselection, gets units inside the box
  (Variables|Default|SetIsMultiSelection false)
  (CallFunction|UnselectAllUnits)
  (CallFunction|UnselectBuilding)
  (bind _multiselectionbox (Variables|Default|GetMultiSelectionBox)
    (:then
      (bind _actors (Default|GetSelectionActors _multiselectionbox))
      (CallFunction|SelectUnitsfromActors _actors)
      (Actor|DestroyActor (Variables|Default|GetMultiSelectionBox)))
    (:else)))

(event Custom|MultiSelectionTick
  ;[1 1 1] Tick event of multiselection to update box transform and size
  (if (Variables|Default|GetIsMultiSelection)
    (bind _multiselectionbox (Variables|Default|GetMultiSelectionBox)
      (:then
        (bind (_location _sizex _sizey) (CallFunction|GetNewMultiSelectionData))
        (Transformation|SetActorLocation _multiselectionbox _location false false)
        (Components|Box|SetBoxExtent (Variables|/Game/Blueprints/Gameplay/GameMode/BP_MultiSelectionBoxd.BP_MultiSelectionBoxd_C|GetBox _multiselectionbox) (Math|Vector|MakeVector _sizex _sizey 5e+02) true))
      (:else))))

(event Custom|ServerMoveUnits
  (params (Location :type Vector) (Units :type Array%20of%20BP%20Master%20Unit%20Object%20References) (TryAttack :type Boolean))
  ;[1 1 1] Server handles requesting units to move
  (for _array_element Units
    (Development|PrintString (Utilities|String|ToString(Boolean) (and (Default|IsFriendly _array_element self) (not (Variables|/Game/Blueprints/Gameplay/Units/BP_MasterUnit.BP_MasterUnit_C|GetDead _array_element)))) true true "(R=0.000000,G=0.065312,B=0.098958,A=1.000000)")
    (if (and (Default|IsFriendly _array_element self) (not (Variables|/Game/Blueprints/Gameplay/Units/BP_MasterUnit.BP_MasterUnit_C|GetDead _array_element)))
      (Default|MovetoLocation _array_element Location TryAttack)
      (Variables|/Game/Blueprints/Gameplay/Units/BP_MasterUnit.BP_MasterUnit_C|SetInCommandAction _array_element true))))

(event Custom|ServerAttackUnit
  (params (TargetUnit :type BP%20Master%20Unit%20Object%20Reference) (Units :type Array%20of%20BP%20Master%20Unit%20Object%20References))
  ;[1 1 1] Server handles requesting units to attack unit
  (for _array_element Units
    (if (and (Default|IsFriendly _array_element self) (not (Variables|/Game/Blueprints/Gameplay/Units/BP_MasterUnit.BP_MasterUnit_C|GetDead _array_element)))
      (Default|AttackUnit _array_element TargetUnit)
      (Variables|/Game/Blueprints/Gameplay/Units/BP_MasterUnit.BP_MasterUnit_C|SetInCommandAction _array_element true))))

(event Custom|ServerAttackBuilding
  (params (TargetBuilding :type BP%20Master%20Building%20Object%20Reference) (Units :type Array%20of%20BP%20Master%20Unit%20Object%20References))
  ;[1 1 1] Server handles requesting units to attack building
  (for _array_element Units
    (if (and (Default|IsFriendly _array_element self) (not (Variables|/Game/Blueprints/Gameplay/Units/BP_MasterUnit.BP_MasterUnit_C|GetDead _array_element)))
      (Default|AttackBuilding _array_element TargetBuilding)
      (Variables|/Game/Blueprints/Gameplay/Units/BP_MasterUnit.BP_MasterUnit_C|SetInCommandAction _array_element true))))

(event Custom|ClientShowEndScreen
  (params (Victory :type Boolean))
  ;[1 1 1] Handles showing end of game screen on client
  (Default|ShowEndScreen (CallFunction|GetHUDRef) Victory))

(event Custom|SelectedBuildingAction
  (params (BuildingAction :type BP%20Master%20Building%20Action%20Class%20Reference))
  ;[1 1 1] Handles selecting building action and sends request to server
  (bind _selectedbuilding (Variables|Default|GetSelectedBuilding)
    (:then
      (CallFunction|ServerSelectedBuildingAction _selectedbuilding BuildingAction))
    (:else)))

(event Custom|ServerSelectedBuildingAction
  (params (Building :type BP%20Master%20Building%20Object%20Reference) (BuildingAction :type BP%20Master%20Building%20Action%20Class%20Reference))
  ;[1 1 1] Server handles building action and calls building to do it
  (Default|StartAction Building BuildingAction))

(event EventBeginPlay
  ;[1 1 1] Sets mode to game and ui and shows mouse cursor
  (if (Pawn|IsLocalPlayerController)
    (Input|SetInputModeGameandUI self 0 "DoNotLock" false)
    (Variables|Default|SetbShowMouseCursor true)))

(event EventTick
  (params (DeltaSeconds :type Float%20%28single-precision%29))
  ;[1 1 1] Handles single selection or multi selection based on time of click
  (if (Pawn|IsLocalPlayerController)
    (CallFunction|MultiSelectionTick)
    (CallFunction|ConstructionTick)))

(event Input|ActionEvents|InputActionSelection
  (params (Key :type Key%20Structure :default "None"))
  (bind (_locationx _locationy) (Game|Player|GetMousePosition))
  ;[1 1 1] Handles single selection or multi selection based on time of click
  (:Pressed
    (bind _hitlocation (CallFunction|GetMouseHitLocation))
    (Variables|Default|SetMultiSelectionStartLocation (.location (Class|KismetMathLibrary|ConvertTransformtoRelative (Transformation|GetActorTransform (CallFunction|GetCameraPawn)) (Math|Transform|MakeTransform _hitlocation "0, 0, 0" "1,1,1"))))
    (Variables|Default|SetMouseMultiSelectionStartLocation (Math|Vector2D|MakeVector2D _locationx _locationy))
    (bind _returnvalue (Utilities|Time|SetTimerbyEvent (EventDispatchers|CreateEvent :!event Custom|StartMultiSelection) (Variables|Default|GetSingleSelectionThreshold)))
    (Variables|Default|SetMultiSelectionTimer _returnvalue))
  (:Released
    (Utilities|FlowControl|Sequence
      (:then_0
        (if (Utilities|Time|IsValidTimerHandle (Variables|Default|GetMultiSelectionTimer))
          (Utilities|Time|ClearandInvalidateTimerbyHandle (Variables|Default|GetMultiSelectionTimer))
          (CallFunction|SingleSelection)
          (else
            (CallFunction|StopMultiSelection))))
      (:then_1
        (if (Variables|Default|GetIsConstructionMode)
          (bind _buildingghost (Variables|Default|GetBuildingGhost)
            (:then
              (CallFunction|ServerBuild (Variables|Default|GetBuildingClass) (Transformation|GetActorLocation _buildingghost))
              (CallFunction|ToggleConstruction false))
            (:else)))))))

(event Input|ActionEvents|InputActionAction
  (params (Key :type Key%20Structure :default "None"))
  ;[1 1 1] Handles action based on what is clicked
  (:Pressed
    (bind _hitactor (CallFunction|GetMouseHitActor))
    (bind _asbp_master_unit (Utilities|Casting|CastToBP_MasterUnit _hitactor)
      (:then
        (if (not (or (Default|IsFriendly _asbp_master_unit self) (Variables|/Game/Blueprints/Gameplay/Units/BP_MasterUnit.BP_MasterUnit_C|GetDead _asbp_master_unit)))
          (CallFunction|ServerAttackUnit _asbp_master_unit (Variables|Default|GetSelectedUnits))))
      (:CastFailed
        (bind _asbp_master_building (Utilities|Casting|CastToBP_MasterBuilding _hitactor)
          (:then
            (if (not (Default|IsFriendly _asbp_master_building self))
              (CallFunction|ServerAttackBuilding _asbp_master_building (Variables|Default|GetSelectedUnits))))
          (:CastFailed
            (bind _hitlocation (CallFunction|GetMouseHitLocation))
            (CallFunction|ServerMoveUnits _hitlocation (Variables|Default|GetSelectedUnits) (Variables|Default|GetIsAPressed))))))))

(event Input|KeyboardEvents|A
  (params (Key :type Key%20Structure :default "None"))
  ;[1 1 1] Handles A pressed state
  (:Pressed
    (Variables|Default|SetIsAPressed true))
  (:Released
    (Variables|Default|SetIsAPressed false)))

(fn ConstructionScript)

(fn GetMouseHitActor
  (bind (_worldlocation _worlddirection) (Game|Player|ConvertMouseLocationToWorldSpace))
  (bind (_outhit _returnvalue) (Collision|LineTraceByChannel _worldlocation (+ _worldlocation (* _worlddirection 1e+05)) "TraceTypeQuery1" false 0 "None"))
  (if _returnvalue
    (return (.HitActor (Collision|BreakHitResult _outhit)))
    (else
      (return 0))))

(fn UnselectAllUnits
  (for _array_element (Variables|Default|GetSelectedUnits)
    (Default|ToggleSelection _array_element false)
    (EventDispatchers|UnbindEventfromDeath _array_element (EventDispatchers|CreateEvent :!event OnSelectedUnitDeath)))
  (Utilities|Array|Clear (Variables|Default|GetSelectedUnits))
  (Default|ClearSelectedUnits (CallFunction|GetHUDRef))
  (return))

(fn SelectUnits
  (params (Units :type Array%20of%20BP%20Master%20Unit%20Object%20References))
  (for _array_element Units
    (Default|ToggleSelection _array_element true)
    (EventDispatchers|BindEventtoDeath _array_element (EventDispatchers|CreateEvent :!event OnSelectedUnitDeath)))
  (Utilities|Array|AppendArray (Variables|Default|GetSelectedUnits) Units)
  (Default|UpdateSelectedUnits (CallFunction|GetHUDRef) (Variables|Default|GetSelectedUnits))
  (return))

(fn GetMouseHitLocation
  (bind (_worldlocation _worlddirection) (Game|Player|ConvertMouseLocationToWorldSpace))
  (bind _outhit (Collision|LineTraceByChannel _worldlocation (+ _worldlocation (* _worlddirection 1e+05)) "TraceTypeQuery1" false 0 "None"))
  (return (Math|Vector|SelectVector (.Location (Collision|BreakHitResult _outhit)) (.TraceEnd (Collision|BreakHitResult _outhit)) (.bBlockingHit (Collision|BreakHitResult _outhit)))))

(fn GetNewMultiSelectionData
  (bind _multiselectionstartlocation (Variables|Default|GetMultiSelectionStartLocation))
  (bind _hitlocation (CallFunction|GetMouseHitLocation))
  (return (Math|Transform|TransformLocation (Transformation|GetActorTransform (CallFunction|GetCameraPawn)) (- (.location (Class|KismetMathLibrary|ConvertTransformtoRelative (Transformation|GetActorTransform (CallFunction|GetCameraPawn)) (Math|Transform|MakeTransform _hitlocation "0, 0, 0" "1,1,1"))) (/ (- (.location (Class|KismetMathLibrary|ConvertTransformtoRelative (Transformation|GetActorTransform (CallFunction|GetCameraPawn)) (Math|Transform|MakeTransform _hitlocation "0, 0, 0" "1,1,1"))) _multiselectionstartlocation) 2.0))) (/ (.X (Math|Vector|BreakVector (- _multiselectionstartlocation (.location (Class|KismetMathLibrary|ConvertTransformtoRelative (Transformation|GetActorTransform (CallFunction|GetCameraPawn)) (Math|Transform|MakeTransform _hitlocation "0, 0, 0" "1,1,1")))))) 2.0) (/ (.Y (Math|Vector|BreakVector (- _multiselectionstartlocation (.location (Class|KismetMathLibrary|ConvertTransformtoRelative (Transformation|GetActorTransform (CallFunction|GetCameraPawn)) (Math|Transform|MakeTransform _hitlocation "0, 0, 0" "1,1,1")))))) 2.0)))

(fn GetCameraPawn
  (bind _asbp_camera_pawn (Utilities|Casting|CastToBP_CameraPawn (Pawn|GetControlledPawn)))
  (return _asbp_camera_pawn))

(fn SelectUnitsfromActors
  (params (Actors :type Array%20of%20Actor%20Object%20References))
  (for _array_element Actors
    (bind _asbp_master_unit (Utilities|Casting|CastToBP_MasterUnit _array_element))
    (Utilities|Array|Add (LocalVariables|GetUnits) _asbp_master_unit))
  (CallFunction|SelectUnits (LocalVariables|GetUnits))
  (return))

(fn OnRepGold
  (Default|CallGoldUpdated (Variables|Default|GetGold)))

(fn GetHUDRef
  (bind _ashud_gameplay (Utilities|Casting|CastToHUD_Gameplay (HUD|GetHUD)))
  (return _ashud_gameplay))

(fn OnSelectedUnitDeath
  (params (Unit :type BP%20Master%20Unit%20Object%20Reference))
  (Default|ToggleSelection Unit false)
  (Utilities|Array|RemoveItem (Variables|Default|GetSelectedUnits) Unit))

(fn SelectBuilding
  (params (Building :type BP%20Master%20Building%20Object%20Reference))
  (bind _output_get (Variables|Default|SetSelectedBuilding Building))
  (Default|ToggleSelection _output_get true)
  (Default|ToggleBuildingHUD (CallFunction|GetHUDRef) true (Variables|Default|GetSelectedBuilding)))

(fn UnselectBuilding
  (bind _selectedbuilding (Variables|Default|GetSelectedBuilding)
    (:then
      (Default|ToggleSelection _selectedbuilding false))
    (:else
      _))
  (Variables|Default|SetSelectedBuilding 0)
  (Default|ToggleBuildingHUD (CallFunction|GetHUDRef) false))

(fn OnRepConstructionBuildings
  (Default|CallUpdatedConstructionBuildings (Variables|Default|GetConstructionBuildings)))