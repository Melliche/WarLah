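; Multi-selection box actor that reports which actors lie within its Box component, with no active event logic of its own.
; GetSelectionActors runs a zero-length multi box trace on the Visibility channel at the actor's location and rotation, using absolute X and Y extents.
; Hit actors are added uniquely to ActorsTmp, which the function returns without clearing it first.
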(event EventBeginPlay)

(event Collision|EventActorBeginOverlap
  (params (OtherActor :type Actor%20Object%20Reference)))

(event EventTick
  (params (DeltaSeconds :type Float%20%28single-precision%29)))

(fn ConstructionScript)

(fn GetSelectionActors
  (bind _returnvalue (Transformation|GetActorLocation))
  (bind _box (Variables|Default|GetBox))
  (bind _boxextent (Variables|/Script/Engine.BoxComponent|GetBoxExtent _box))
  (bind _outhits (Class|KismetSystemLibrary|BoxTraceMulti _returnvalue _returnvalue (Math|Vector|MakeVector (Math|Float|Absolute(Float) (.x _boxextent)) (Math|Float|Absolute(Float) (.y _boxextent)) (.z _boxextent)) (Transformation|GetActorRotation) "TraceTypeQuery1" false 0 "None" true))
  (for _array_element _outhits
    (Utilities|Array|AddUnique (LocalVariables|GetActorsTmp) (.hitactor _array_element)))
  (return (LocalVariables|GetActorsTmp)))