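; Multiplayer game mode that runs a clan-based match, from waiting screen to last town hall standing.
; PostLogin assigns joining controllers one of three clans, then at the target player count spawns and possesses camera pawns at clan-matched player starts.
; Town hall EndPlay events drive elimination: the owner gets a defeat screen, and the last clan standing gets victory.
; A short timer follows the win, with server travel used to restart the map.
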(event Custom|SpawnPC
  (params (PC :type PC%20Gameplay%20Object%20Reference))
  (bind _clan (Variables|/Game/Blueprints/Gameplay/GameMode/PC_Gameplay.PC_Gameplay_C|GetClan PC))
  (bind _transform (CallFunction|GetPlayerStart _clan))
  ;[1 1 1] Handles spawning camera pawn for player controller
  (bind _returnvalue (Game|SpawnActorfromClass "/Game/Blueprints/Gameplay/GameMode/BP_CameraPawn.BP_CameraPawn_C" (Math|Transform|MakeTransform (.location _transform) (.rotation _transform) "1,1,1") "AdjustIfPossibleButAlwaysSpawn" 0 0))
  (Pawn|Possess PC _returnvalue))

(event EventBeginPlay
  ;[1 1 1] Init
  (bind _outactors (Actor|GetAllActorsOfClass "/Game/Blueprints/Gameplay/GameMode/BP_PlayerStart.BP_PlayerStart_C"))
  (Variables|Default|SetPlayerStarts _outactors)
  (bind _outactors_2 (Actor|GetAllActorsOfClass "/Game/Blueprints/Gameplay/Buildings/BP_Building_TownHall.BP_Building_TownHall_C"))
  (bind _output_get (Variables|Default|SetTownHalls _outactors_2))
  (for _array_element _output_get
    (Game|AssignOnEndPlay _array_element (EventDispatchers|CreateEvent :!event OnTownHallDestroyed))))

(event EventPostLogin
  (params (NewPlayer :type Player%20Controller%20Object%20Reference))
  ;[1 1 1] Handles receiving joining player controllers and starting match if possible
  (if (not (Variables|Default|GetMatchStarted))
    (bind _aspc_gameplay (Utilities|Casting|CastToPC_Gameplay NewPlayer))
    (bind _returnvalue (Utilities|Array|Add (Variables|Default|GetPCs) _aspc_gameplay))
    (Default|ClientToggleWaitingScreen _aspc_gameplay true)
    (Variables|/Game/Blueprints/Gameplay/GameMode/PC_Gameplay.PC_Gameplay_C|SetClan _aspc_gameplay (Utilities|Enum|ByteToEnumE_Clans (Math|Conversions|ToByte(Integer) (Math|Integer|%(Integer) _returnvalue 3))))
    (if (== (Utilities|Array|Length (Variables|Default|GetPCs)) (Variables|Default|GetTotalPlayers))
      (Variables|Default|SetMatchStarted true)
      (for _array_element (Variables|Default|GetPCs)
        (CallFunction|SpawnPC _array_element)
        (Default|ClientToggleWaitingScreen _array_element false)))))

(fn ConstructionScript)

(fn GetPlayerStart
  (params (Clan :type E_Clans%20Enum :default "NewEnumerator0"))
  (for _array_element (Variables|Default|GetPlayerStarts)
    (if (Utilities|Enum|Equal(Enum) (Variables|/Game/Blueprints/Gameplay/GameMode/BP_PlayerStart.BP_PlayerStart_C|GetClan _array_element) Clan)
      (return (Math|Transform|MakeTransform (.location (Transformation|GetActorTransform _array_element)) (.rotation (Transformation|GetActorTransform _array_element)) "1,1,1"))))
  (return ""))

(fn OnTownHallDestroyed
  (params (Actor :type Actor%20Object%20Reference) (EndPlayReason :type EEndPlayReason%20Enum :default "Destroyed"))
  (bind _asbp_building_town_hall (Utilities|Casting|CastToBP_Building_TownHall Actor))
  (Utilities|Array|RemoveItem (Variables|Default|GetTownHalls) _asbp_building_town_hall)
  (Utilities|IsValid (CallFunction|GetPCOfClan (Variables|/Game/Blueprints/Gameplay/Buildings/BP_MasterBuilding.BP_MasterBuilding_C|GetClan _asbp_building_town_hall))
    (:Is%20Valid
      (Default|ClientShowEndScreen (CallFunction|GetPCOfClan (Variables|/Game/Blueprints/Gameplay/Buildings/BP_MasterBuilding.BP_MasterBuilding_C|GetClan _asbp_building_town_hall)) false))
    (:Is%20Not%20Valid
      _))
  (bind (_ended _winnerpc) (CallFunction|CheckGameEnded))
  (if _ended
    (Default|ClientShowEndScreen _winnerpc true)
    (Utilities|Time|SetTimerbyEvent (EventDispatchers|CreateEvent :!event RestartGame) 3.0)))

(fn GetPCOfClan
  (params (Clan :type E_Clans%20Enum :default "NewEnumerator0"))
  (for _array_element (Variables|Default|GetPCs)
    (Utilities|IsValid _array_element
      (:Is%20Valid
        (if (Utilities|Enum|Equal(Enum) (Variables|/Game/Blueprints/Gameplay/GameMode/PC_Gameplay.PC_Gameplay_C|GetClan _array_element) Clan)
          (return _array_element)))))
  (return 0))

(fn CheckGameEnded
  (bind _townhalls (Variables|Default|GetTownHalls))
  (if (== (Utilities|Array|Length _townhalls) 1)
    (return true (CallFunction|GetPCOfClan (Variables|/Game/Blueprints/Gameplay/Buildings/BP_MasterBuilding.BP_MasterBuilding_C|GetClan (Utilities|Array|Get(acopy) _townhalls))))
    (else
      (return false 0))))

(fn RestartGame
  (Development|ExecuteConsoleCommand "ServerTravel /Game/Maps/GameplayMap" 0))