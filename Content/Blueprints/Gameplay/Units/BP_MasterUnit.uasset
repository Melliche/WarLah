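; Base RTS-style unit character with clan allegiance, selection highlight, camera-facing health bar and replicated health and death.
; Move and attack commands write target and state to the AI blackboard for a behavior tree.
; Attacks spawn projectiles or sphere-overlap melee hits and alert nearby units, while damaged units retaliate unless under command.
; Death stops AI and movement, ragdolls the mesh through OnRep, then destroys the actor after a delay.
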(event Custom|UpdateHealth3D
  ;[1 1 1] Handles updating health widget
  (Networking|CanExecuteCosmeticEvents
    (:True
      (bind _aswbp_health_3d (Utilities|Casting|CastToWBP_Health3D (UserInterface|GetUserWidgetObject (Variables|Default|GetHealthWidget))))
      (Default|UpdateHealth _aswbp_health_3d (Variables|Default|GetCurrentHealth) (Variables|Default|GetMaxHealth)))))

(event Custom|LookAtActor
  (params (TargetActor :type Actor%20Object%20Reference))
  ;[1 1 1] Handles smoothly rotating towards target
  (Variables|Default|SetActorRotationTemp (Transformation|GetActorRotation))
  (bind _alpha (Timeline|LookAtActorRotation PlayFromStart)
    (:Update
      (Utilities|IsValid TargetActor
        (:Is%20Valid
          (Transformation|SetActorRotation (Math|Rotator|Lerp(Rotator) (Math|Rotator|MakeRotator (.roll (Variables|Default|GetActorRotationTemp)) (.pitch (Variables|Default|GetActorRotationTemp)) (.yaw (Variables|Default|GetActorRotationTemp))) (Math|Rotator|MakeRotator (.roll (Variables|Default|GetActorRotationTemp)) (.pitch (Variables|Default|GetActorRotationTemp)) (.yaw (Math|Rotator|FindLookatRotation (Transformation|GetActorLocation) (Transformation|GetActorLocation TargetActor)))) _alpha true)))))
    (:Finished
      (Default|CallCompletedLookat))))

(event Custom|AttackAlert
  ;[1 1 1] Alerts nearby units within the specified distance
  (bind (_outactors _returnvalue) (Collision|SphereOverlapActors (Transformation|GetActorLocation) (Variables|Default|GetAttackAlertRadius) (Utilities|Array|MakeArray "ObjectTypeQuery3") "BP_MasterUnit_C" (Utilities|Array|MakeArray self)))
  (if _returnvalue
    (for _array_element _outactors
      (bind _asbp_master_unit (Utilities|Casting|CastToBP_MasterUnit _array_element))
      (if (not (Variables|BP_MasterUnit_C|GetInCommandAction _asbp_master_unit))
        (CallFunction|Alert _asbp_master_unit self)))))

(event Custom|MoveToLocation
  (params (TargetLocation :type Vector) (TryAttack :type Boolean))
  (bind _self self)
  (bind _returnvalue (AI|GetBlackboard _self))
  ;[1 1 1] Sets move to location to behavior tree
  (AI|Components|Blackboard|SetValueasVector _returnvalue (Utilities|Name|MakeLiteralName "TargetLocation") TargetLocation)
  (AI|Components|Blackboard|SetValueasEnum _returnvalue (Utilities|Name|MakeLiteralName "State") (select TryAttack "NewEnumerator3" "NewEnumerator1")))

(event Custom|AttackUnit
  (params (TargetUnit :type BP%20Master%20Unit%20Object%20Reference))
  (bind _self self)
  (bind _returnvalue (AI|GetBlackboard _self))
  ;[1 1 1] Sets attack unit to behavior tree
  (AI|Components|Blackboard|SetValueasObject _returnvalue (Utilities|Name|MakeLiteralName "TargetActor") TargetUnit)
  (AI|Components|Blackboard|SetValueasEnum _returnvalue (Utilities|Name|MakeLiteralName "State") (Utilities|Enum|LiteralenumE_UnitStates "NewEnumerator2")))

(event Custom|MulticastMontage
  (params (AnimMontage :type Anim%20Montage%20Object%20Reference))
  ;[1 1 1] Handles playing anim montage on server and all clients
  (Animation|PlayAnimMontage AnimMontage 1.0 "None"))

(event Custom|AttackCollision
  (bind _actor (CallFunction|GetTargetActor))
  ;[1 1 1] Handles applying damage based on a sphere overlap function in front of the unit
  (CallFunction|AttackAlert)
  (if (Variables|Default|GetIsRangeAttack)
    (Utilities|IsValid _actor
      (:Is%20Valid
        (Game|SpawnActorfromClass (Variables|Default|GetRangeAttackProjectile) (Math|Transform|MakeTransform (Transformation|GetWorldLocation (Variables|Default|GetProjectileSpawnLocation)) (Math|Rotator|FindLookatRotation (Transformation|GetActorLocation) (Transformation|GetActorLocation _actor)) "1,1,1") "AlwaysSpawn" self (Variables|Default|GetAttackDamage) _actor 0)))
    (else
      (bind _outactors (Collision|SphereOverlapActors (+ (Transformation|GetActorLocation) (* (Transformation|GetActorForwardVector) 5e+01)) 25.0 (Utilities|Array|MakeArray "ObjectTypeQuery3" "ObjectTypeQuery1" "ObjectTypeQuery2") "/Script/Engine.Actor" (Utilities|Array|MakeArray self)))
      (for _array_element _outactors
        (bind _clan (Class|BPIGameplayLibrary|GetClan(Message) _array_element))
        (if (Utilities|Enum|NotEqual(Enum) _clan (Variables|Default|GetClan))
          (Game|Damage|ApplyDamage _array_element (Variables|Default|GetAttackDamage) 0 self))))))

(event Custom|AttackBuilding
  (params (Building :type BP%20Master%20Building%20Object%20Reference))
  (bind _self self)
  (bind _returnvalue (AI|GetBlackboard _self))
  ;[1 1 1] Sets attack building to behavior tree
  (AI|Components|Blackboard|SetValueasObject _returnvalue (Utilities|Name|MakeLiteralName "TargetActor") Building)
  (AI|Components|Blackboard|SetValueasEnum _returnvalue (Utilities|Name|MakeLiteralName "State") (Utilities|Enum|LiteralenumE_UnitStates "NewEnumerator2")))

(event Custom|StopLookAt
  (bind _actorrotationtemp (Variables|Default|GetActorRotationTemp))
  ;[1 1 1] Handles smoothly rotating towards target
  (bind _alpha (Timeline|LookAtActorRotation Stop)
    (:Update
      (Utilities|IsValid (stale Custom|LookAtActor TargetActor)
        (:Is%20Valid
          (Transformation|SetActorRotation (Math|Rotator|Lerp(Rotator) (Math|Rotator|MakeRotator (.roll _actorrotationtemp) (.pitch _actorrotationtemp) (.yaw _actorrotationtemp)) (Math|Rotator|MakeRotator (.roll _actorrotationtemp) (.pitch _actorrotationtemp) (.yaw (Math|Rotator|FindLookatRotation (Transformation|GetActorLocation) (Transformation|GetActorLocation (stale Custom|LookAtActor TargetActor))))) _alpha true)))))
    (:Finished
      (Default|CallCompletedLookat))))

(event Custom|CombatState
  ;[1 1 1] Enables combat state and resets after specified delay
  (Utilities|Time|ClearandInvalidateTimerbyHandle (Variables|Default|GetCombatStateResetTimer))
  (bind _returnvalue (Utilities|Time|SetTimerbyEvent (EventDispatchers|CreateEvent :!event HandleCombatState) 0.25 true))
  (Variables|Default|SetHandleCombatStateTimer _returnvalue)
  (bind _returnvalue_2 (Utilities|Time|SetTimerbyEvent (delegate Custom|CombatStateReset) (Variables|Default|GetCombatStateResetDelay)))
  (Variables|Default|SetCombatStateResetTimer _returnvalue_2))

(event Custom|CombatStateReset
  ;[1 1 1] Enables combat state and resets after specified delay
  (Utilities|Time|ClearandInvalidateTimerbyHandle (Variables|Default|GetHandleCombatStateTimer)))

(event Game|Damage|EventAnyDamage
  (params (Damage :type Float%20%28single-precision%29) (DamageType :type Damage%20Type%20Object%20Reference) (InstigatedBy :type Controller%20Object%20Reference) (DamageCauser :type Actor%20Object%20Reference))
  ;[1 1 1] Handles receiving damage and death if no health
  (if (not (Variables|Default|GetDead))
    (Utilities|HandleHitReaction DamageCauser)
    (bind _output_get (Variables|Default|SetCurrentHealth (Math|Float|Clamp(Float) (- (Variables|Default|GetCurrentHealth) Damage) 0.0 (Variables|Default|GetMaxHealth))))
    (if (== _output_get 0.0)
      (Variables|Default|SetDead true)
      (Components|Activation|Deactivate (Variables|Character|GetCharacterMovement))
      (AI|Logic|StopLogic (Variables|/Script/AIModule.AIController|GetBrainComponent (AI|GetAIController self)) "Death")
      (Utilities|FlowControl|Delay 3e+01)
      (Actor|DestroyActor))))

(event EventTick
  (params (DeltaSeconds :type Float%20%28single-precision%29))
  (bind _healthwidget (Variables|Default|GetHealthWidget))
  ;[1 1 1] Handles rotating health widget towards camera when possible (If not dedicated server)
  (Networking|CanExecuteCosmeticEvents
    (:True
      (Transformation|SetWorldRotation _healthwidget (Math|Rotator|FindLookatRotation (Transformation|GetWorldLocation _healthwidget) (Transformation|GetActorLocation (Game|GetPlayerCameraManager 0))) false false))))

(event EventBeginPlay
  ;[1 1 1] Init
  (CallFunction|UpdateHealth3D))

(fn ConstructionScript)

(fn ToggleSelection
  (params (Show :type Boolean))
  (bind _output_get (Variables|Default|SetIsSelected Show))
  (if _output_get
    (Rendering|Material|SetMaterial (Variables|Default|GetSelectionMesh) 0 (select (CallFunction|IsFriendly (.AsPC%20Gameplay (Utilities|Casting|CastToPC_Gameplay (Game|GetPlayerController 0)))) "/Game/Materials/M_SelectedUnit_Friendly.M_SelectedUnit_Friendly" "/Game/Materials/M_SelectedUnit_Enemy.M_SelectedUnit_Enemy")))
  (Rendering|SetVisibility (Variables|Default|GetSelectionMesh) (Variables|Default|GetIsSelected) false))

(fn IsFriendly
  (params (PC :type PC%20Gameplay%20Object%20Reference))
  (return (Utilities|Enum|Equal(Enum) (Variables|/Game/Blueprints/Gameplay/GameMode/PC_Gameplay.PC_Gameplay_C|GetClan PC) (Variables|Default|GetClan))))

(fn OnRepCurrentHealth
  (Default|CallUpdateHealth (Variables|Default|GetCurrentHealth) (Variables|Default|GetMaxHealth))
  (CallFunction|UpdateHealth3D))

(fn OnRepDead
  (if (Variables|Default|GetDead)
    (Default|CallDeath self)
    (Physics|SetSimulatePhysics (Variables|Character|GetMesh) true)
    (Collision|SetCollisionEnabled (Variables|Collision|GetCapsuleComponent) "NoCollision")
    (Collision|SetCollisionResponsetoChannel (Variables|Character|GetMesh) "ECC_Pawn" "ECR_Ignore")
    (Networking|CanExecuteCosmeticEvents
      (:True
        (Rendering|SetVisibility (Variables|Default|GetHealthWidget) false false)))))

(fn GetTargetActor
  (bind _asactor (Utilities|Casting|CastToActor (AI|Components|Blackboard|GetValueasObject (AI|GetBlackboard self) (Utilities|Name|MakeLiteralName "TargetActor")))
    (:then
      (return _asactor))
    (:CastFailed
      (return 0))))

(fn FindClosestAttackUnit
  (bind (_outactors _returnvalue) (Collision|SphereOverlapActors (Transformation|GetActorLocation) 1e+03 (Utilities|Array|MakeArray "ObjectTypeQuery3") "BP_MasterUnit_C" (Utilities|Array|MakeArray self)))
  (if _returnvalue
    (for _array_element _outactors
      (bind _asbp_master_unit (Utilities|Casting|CastToBP_MasterUnit _array_element))
      (if (and (not (Variables|BP_MasterUnit_C|GetDead _asbp_master_unit)) (Utilities|Enum|NotEqual(Enum) (Variables|BP_MasterUnit_C|GetClan _asbp_master_unit) (Variables|Default|GetClan)))
        (if (or (LocalVariables|GetIsFirst) (< (Math|Vector|Distance(Vector) (Transformation|GetActorLocation _asbp_master_unit) (Transformation|GetActorLocation)) (LocalVariables|GetClosestDistance)))
          (LocalVariables|SetIsFirst false)
          (LocalVariables|SetClosestUnit _asbp_master_unit)
          (LocalVariables|SetClosestDistance (Math|Vector|Distance(Vector) (Transformation|GetActorLocation _asbp_master_unit) (Transformation|GetActorLocation))))))
    (return (Utilities|IsValid (LocalVariables|GetClosestUnit)) (LocalVariables|GetClosestUnit))
    (else
      (return false 0))))

(fn HandleCombatState
  (Utilities|IsValid (CallFunction|GetTargetActor)
    (:Is%20Valid
      (return))
    (:Is%20Not%20Valid
      (bind (_found _unit) (CallFunction|FindClosestAttackUnit))
      (if _found
        (CallFunction|AttackUnit _unit)
        (return)
        (else
          (return))))))

(fn Alert
  (params (Unit :type BP%20Master%20Unit%20Object%20Reference))
  (if (Math|Boolean|ANDBoolean (Utilities|Enum|NotEqual(Enum) (Variables|BP_MasterUnit_C|GetClan Unit) (Variables|Default|GetClan)) (not (Variables|BP_MasterUnit_C|GetDead Unit)) (not (Variables|Default|GetDead)))
    (if (not (== (Class|BlackboardComponent|GetValueasEnum (AI|GetBlackboard self) (Utilities|Name|MakeLiteralName "State")) (Utilities|Enum|LiteralenumE_UnitStates "NewEnumerator2")))
      (CallFunction|AttackUnit Unit))))

(fn GetClan
  (return (Variables|Default|GetClan)))

(fn GetInteractionDistance
  (return 1.5e+02))

(fn IsDead
  (return (Variables|Default|GetDead)))